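; BP_Explosive is an explosive actor that detonates once when it takes any damage.
; The blast spawns particles, sound, radial damage and a distance-based camera shake, then hides the mesh and disables its collision.
; An option credits the shooter as damage causer, sparing them and awarding points.
; Optional slow motion clears the reset flag on all other explosives, so only the latest blast restores normal time after a delay.
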(event Game|Damage|EventAnyDamage
  (params (Damage :type Float%20%28single-precision%29) (DamageType :type Damage%20Type%20Object%20Reference) (InstigatedBy :type Controller%20Object%20Reference) (DamageCauser :type Actor%20Object%20Reference))
  ;[0 0 0] Explosion event
  ;;[1 1 1] Any damage is caused
  ;;[1 1 1] If shooter is damage causer, explosion will not hurt player and will get points for everything the blast will damage/kill
  (Variables|Default|SetDamageCauser (select (Variables|Default|GetShooterAsDamageCauser) DamageCauser 0))
  ;;[1 1 1] Explode
  (Utilities|FlowControl|DoOnce false
    (:Completed
      ;;[1 1 1] Spawn particle system
      (Effects|SpawnEmitteratLocation "/Game/FPSK/Particles/PS_Explosion.PS_Explosion" (Transformation|GetActorLocation))
      ;;[1 1 1] Play sound effect at location
      (Audio|PlaySoundatLocation "/Game/FPSK/Sounds/WAV_NukeExplosion.WAV_NukeExplosion" (Transformation|GetActorLocation) "0, 0, 0" 1.0 1.0 0.0 "/Game/FPSK/Sounds/Audio/Attenuation_ReallyFarRange.Attenuation_ReallyFarRange")
      ;;[1 1 1] Apply radial damage
      (Game|Damage|ApplyRadialDamage (Variables|Default|GetDamage) (+ (Transformation|GetActorLocation) "0, 0,1.000000") (Variables|Default|GetDamageRadius) 0 0 (Variables|Default|GetDamageCauser) 0 false "ECC_Visibility")
      ;;[1 1 1] Play camera shake based on distance
      (Camera|PlayWorldCameraShake "/Game/FPSK/Blueprint/Widget/BP_CS_Explosion.BP_CS_Explosion_C" (Transformation|GetActorLocation) 0.0 2e+04 1e+01 true)
      ;;[1 1 1] Hide and turn off collision of mesh
      (Development|SetHiddeninGame (Variables|Default|GetExplosiveMesh) true false)
      (Collision|SetCollisionEnabled (Variables|Default|GetExplosiveMesh) "NoCollision")
      ;;[1 1 1] Turn on temporary slow motion effect if desired
      (if (Variables|Default|GetSlowMotion)
        ;;[1 1 1] Prevent previous explosives to return time dilation
        (bind _outactors (Actor|GetAllActorsOfClass "BP_Explosive_C"))
        (for _array_element _outactors
          (Variables|BP_Explosive_C|SetReturnTimeDilation _array_element false))
        (Variables|Default|SetReturnTimeDilation true)
        ;;[1 1 1] Set slow motion on, then to normal after a delay
        (Utilities|Time|SetGlobalTimeDilation 0.4)
        (Utilities|FlowControl|Delay 2.0)
        (if (Variables|Default|GetReturnTimeDilation)
          (Utilities|Time|SetGlobalTimeDilation 1.0))))))

(fn ConstructionScript)