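; Physics soda bottle hanging on a cord that sprays and leaks when shot or hit by explosions.
; Construction script optionally randomizes soda color, cap color and cord length, sets constraint limits and runs an editor alignment tool.
; BeginPlay jostles the bottle; radial damage also pushes it.
; Damage spawns tinted streams and starts LeakBottle, a delayed self-calling loop fading color and opacity, then disabling further sprays and removing the audio.
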(event Custom|LeakBottle
  ;[0 0 0] Leak Bottle Event
  ;;[1 1 1] Gradually target leaked alpha
  (Variables|Default|SetLeakAlpha (Math|Interpolation|FInterpTo (Variables|Default|GetLeakAlpha) 1.0 (Utilities|Time|GetWorldDeltaSeconds) 5.0))
  ;;[1 1 1] Gradually target leaked opacity
  (bind _output_get (Variables|SodaSettings|SetSodaOpacity (Math|Float|Lerp (Variables|SodaSettings|GetSodaLeakedOpacity) (Variables|SodaSettings|GetSodaOpacity) (Variables|Default|GetLeakAlpha))))
  (Rendering|Material|SetScalarParameterValueonMaterials (Variables|Default|GetSoda) "Opacity" _output_get)
  ;;[1 1 1] Gradually target leaked color
  (bind _output_get_2 (Variables|SodaSettings|SetSodaColor (Math|Color|Lerp(LinearColor) (Variables|SodaSettings|GetSodaColor) "(R=1.000000,G=1.000000,B=1.000000,A=1.000000)" (Variables|Default|GetLeakAlpha))))
  (Rendering|Material|SetVectorParameterValueonMaterials (Variables|Default|GetSoda) "SodaColor" (Math|Conversions|ToVector(LinearColor) _output_get_2))
  ;;[1 1 1] If opacity and color of soda is not at target
  (if (not (Math|Float|NearlyEqual(Float) (Variables|Default|GetLeakAlpha) 1.0 0.1))
    ;;[1 1 1] Loop leak bottle event
    (Utilities|FlowControl|Delay 0.1)
    (CallFunction|LeakBottle)
    (else
      ;;[1 1 1] Set leaked state and change physics material of soda so water particles do not spawn
      (Utilities|FlowControl|DoOnce false
        (:Completed
          (Variables|Default|SetLeaked true)
          (Class|PrimitiveComponent|SetPhysMaterialOverride (Variables|Default|GetSoda) "/Game/FPSK/Physics/PM_Default.PM_Default")
          ;;[1 1 1] Destroy spray audio component
          (Components|DestroyComponent (Variables|Default|GetSprayLoop)))))))

(event EventBeginPlay
  ;[0 0 0] Begin Play events
  ;;[1 1 1] Randomly shake soda bottle physics
  (Physics|AddRadialImpulse (Variables|Default|GetSoda) (+ (Transformation|GetWorldLocation (Variables|Default|GetSoda)) (Math|Vector|MakeVector (Math|Random|RandomFloatinRange -1e+01 1e+01) (Math|Random|RandomFloatinRange -1e+01 1e+01) (Math|Random|RandomFloatinRange -1e+01 1e+01))) 5e+01 5e+01 "RIF_Constant" true))

(event Game|Damage|EventPointDamage
  (params (Damage :type Float%20%28single-precision%29) (DamageType :type Damage%20Type%20Object%20Reference) (HitLocation :type Vector :default "0, 0, 0") (HitNormal :type Vector :default "0, 0, 0") (HitComponent :type Primitive%20Component%20Object%20Reference) (BoneName :type Name :default "None") (ShotFromDirection :type Vector :default "0, 0, 0") (InstigatedBy :type Controller%20Object%20Reference) (DamageCauser :type Actor%20Object%20Reference) (HitInfo :type Hit%20Result%20Structure%20%28by%20ref%29))
  (bind (_bblockinghit _binitialoverlap _time _distance _location _impactpoint _normal) (Collision|BreakHitResult HitInfo))
  ;[0 0 0] Destruction events
  ;;[1 1 1] Spawn stream particle
  (if (not (Variables|Default|GetLeaked)) ; Only if there is currently soda in bottle
    (bind _returnvalue (Effects|SpawnEmitterAttached "/Game/FPSK/Particles/PS_WaterStream.PS_WaterStream" (Variables|Default|GetSoda) "None" _location (Math|Rotator|MakeRotfromZ _normal) "1.000000,1.000000,1.000000" "KeepWorldPosition"))
    ;;[1 1 1] Set color of stream
    (Effects|Components|ParticleSystem|SetVectorParameter _returnvalue "SodaColor" (Math|Conversions|ToVector(LinearColor) (Variables|SodaSettings|GetSodaColor)))
    ;;[1 1 1] Start leaking bottle
    (Utilities|FlowControl|DoOnce false
      (:Completed
        (Audio|Components|Audio|SetVolumeMultiplier (Variables|Default|GetSprayLoop) 1.0 :!class /Script/Engine.AudioComponent)
        (CallFunction|LeakBottle)))))

(event Game|Damage|EventRadialDamage
  (params (DamageReceived :type Float%20%28single-precision%29) (DamageType :type Damage%20Type%20Object%20Reference) (Origin :type Vector :default "0, 0, 0") (HitInfo :type Hit%20Result%20Structure%20%28by%20ref%29) (InstigatedBy :type Controller%20Object%20Reference) (DamageCauser :type Actor%20Object%20Reference))
  ;[0 0 0] Destruction events
  ;;[1 1 1] Apply radial physics from explosions
  (Physics|AddRadialImpulse (Variables|Default|GetSoda) Origin 1e+03 DamageReceived "RIF_Constant" true)
  ;;[1 1 1] Spawn water particle
  (if (not (Variables|Default|GetLeaked)) ; Only if there is currently soda in bottle
    (Utilities|FlowControl|DoOnce false
      (:Completed
        (Effects|SpawnEmitterAttached "/Game/FPSK/Particles/PS_WaterHit.PS_WaterHit" (Variables|Default|GetSoda) "SodaCenter" "0, 0, 0" "0, 0, 0" "3.000000,3.000000,3.000000" "SnapToTarget")
        ;;[1 1 1] Spawn stream particle from soda center
        (bind _returnvalue (Effects|SpawnEmitterAttached "/Game/FPSK/Particles/PS_WaterStream.PS_WaterStream" (Variables|Default|GetSoda) "SodaCenterOutside" "0, 0, 0" "0, 0, 0" "1.000000,1.000000,1.000000" "SnapToTarget"))
        ;;[1 1 1] Set color of stream
        (Effects|Components|ParticleSystem|SetVectorParameter _returnvalue "SodaColor" (Math|Conversions|ToVector(LinearColor) (Variables|SodaSettings|GetSodaColor)))
        ;;[1 1 1] Start leaking bottle
        (Utilities|FlowControl|DoOnce false
          (:Completed
            (Audio|Components|Audio|SetVolumeMultiplier (Variables|Default|GetSprayLoop) 1.0 :!class /Script/Engine.AudioComponent)
            (CallFunction|LeakBottle)))))))

(fn ConstructionScript
  (Utilities|FlowControl|Sequence
    (:then_0
      ;[0 0 0] Randomize color and cord length
      (Utilities|FlowControl|Sequence
        (:then_0
          ;;[1 1 1] Randomize Soda Color
          (if (Variables|SodaSettings|GetRandomizeSodaColor)
            (bind _output_get (Variables|Default|SetSodaColorSeed (Math|Random|RandomInteger 256)))
            (Variables|SodaSettings|SetSodaColor (Utilities|Struct|MakeLinearColor (Math|Random|RandomFloatinRangefromStream 0.0 1.0 (Math|Random|MakeRandomStream _output_get)) (Math|Random|RandomFloatinRangefromStream 0.0 1.0 (Math|Random|MakeRandomStream _output_get)) (Math|Random|RandomFloatinRangefromStream 0.0 1.0 (Math|Random|MakeRandomStream _output_get)) 1.0))
            (Variables|SodaSettings|SetRandomizeSodaColor false)))
        (:then_1
          ;;[1 1 1] Randomize Cap Color
          (if (Variables|SodaSettings|GetRandomizeCapColor)
            (bind _output_get_2 (Variables|Default|SetCapSodaColorSeed (Math|Random|RandomInteger 256)))
            (Variables|SodaSettings|SetCapColor (Utilities|Struct|MakeLinearColor (Math|Random|RandomFloatinRangefromStream 0.0 1.0 (Math|Random|MakeRandomStream _output_get_2)) (Math|Random|RandomFloatinRangefromStream 0.0 1.0 (Math|Random|MakeRandomStream _output_get_2)) (Math|Random|RandomFloatinRangefromStream 0.0 1.0 (Math|Random|MakeRandomStream _output_get_2)) 1.0))
            (Variables|SodaSettings|SetRandomizeCapColor false)))
        (:then_2
          ;;[1 1 1] Randomize Cord Length
          (if (Variables|SodaSettings|GetRandomizeCordLength)
            (bind _output_get_3 (Variables|Default|SetCapSodaColorSeed (Math|Random|RandomInteger 256)))
            (Variables|SodaSettings|SetCordLength (Math|Random|RandomFloatinRangefromStream 25.0 (Variables|SodaSettings|GetMaximumRandomCordLength) (Math|Random|MakeRandomStream _output_get_3)))
            (Variables|SodaSettings|SetRandomizeCordLength false)))))
    (:then_1
      ;[0 0 0] Construct Bottle
      ;;[1 1 1] Set color and opacity of soda
      (Rendering|Material|SetVectorParameterValueonMaterials (Variables|Default|GetSoda) "SodaColor" (Math|Vector|MakeVector (.R (Utilities|Struct|BreakLinearColor (Variables|SodaSettings|GetSodaColor))) (.G (Utilities|Struct|BreakLinearColor (Variables|SodaSettings|GetSodaColor))) (.B (Utilities|Struct|BreakLinearColor (Variables|SodaSettings|GetSodaColor)))))
      (Rendering|Material|SetVectorParameterValueonMaterials (Variables|Default|GetSoda) "Color" (Math|Vector|MakeVector (.R (Utilities|Struct|BreakLinearColor (Variables|SodaSettings|GetCapColor))) (.G (Utilities|Struct|BreakLinearColor (Variables|SodaSettings|GetCapColor))) (.B (Utilities|Struct|BreakLinearColor (Variables|SodaSettings|GetCapColor)))))
      (Rendering|Material|SetScalarParameterValueonMaterials (Variables|Default|GetSoda) "Opacity" (Variables|SodaSettings|GetSodaOpacity))
      ;;[1 1 1] Set physics and cord length
      (Variables|/Script/CableComponent.CableComponent|SetCableLength (Variables|Default|GetCable) 1.0)
      (Class|PhysicsConstraintComponent|SetLinearXLimit (Variables|Default|GetPhysicsConstraint) "LCM_Limited" (Variables|SodaSettings|GetCordLength))
      (Class|PhysicsConstraintComponent|SetLinearYLimit (Variables|Default|GetPhysicsConstraint) "LCM_Limited" (Variables|SodaSettings|GetCordLength))
      (Class|PhysicsConstraintComponent|SetLinearZLimit (Variables|Default|GetPhysicsConstraint) "LCM_Limited" (Variables|SodaSettings|GetCordLength)))
    (:then_2
      ;[0 0 0] Alignment tool for easy alignment in editor
      (Utilities|AlignTool (Variables|AlignmentTool|GetAlignToReference) (Variables|AlignmentTool|GetAlignment)))))