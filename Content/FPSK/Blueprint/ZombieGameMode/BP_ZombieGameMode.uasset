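; Zombie wave-survival game mode that runs waves, kill goals and timed intermissions, announcing wave starts and completion through player HUD animations and sounds.
; WaveSpawn loops on a delay, spawning zombies at random available spawn points up to a live cap, with stats and silhouette color scaled by wave.
; KillCheck completes the wave once the goal is met and no live zombies remain.
; WaveSpawn, KillCheck and BeginIntermission rely on external triggers.
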(event Custom|BeginNextWave
  ;[0 0 0] Begin Next Wave event
  (Variables|Default|SetKillCount 0)
  (Variables|Default|SetIntermission false)
  (Variables|Default|SetIntermissionCheck false)
  (Variables|Default|SetCompleteString "")
  (Math|Integer|IncrementInt (Variables|Default|GetWave)
    (:%20%20
      (CallFunction|WaveDisplayPlayAnimation)
      (Audio|PlaySound2D "/Game/FPSK/Sounds/WAV_WaveStinger.WAV_WaveStinger"))))

(event Custom|WaveSpawn
  ;[0 0 0] Wave Spawn
  (Variables|Default|SetWaveActive true)
  (Utilities|SetWaveSettings (Math|Integer|Clamp(Integer) (+ 5 (Variables|Default|GetWave)) 5 20) 2.0)
  (Utilities|SpawnMacro (+ 5 (Math|Integer|Clamp(Integer) (+ 5 (/ (+ (Variables|Default|GetWave) 1) 2)) 5 20))))

(event Custom|KillCheck
  ;[0 0 0] Kill Check
  ;;[1 1 1] If kill count is acheived
  (Math|Integer|CompareInt (Variables|Default|GetKillCount) (Variables|Default|GetKillGoal)
    (:>
      _)
    (:==
      _))
  ;;[1 1 1] Check if no live targets left
  (Utilities|LiveTargetCountMacro
    (:Out
      ;;[1 1 1] Complete wave and play animation
      (Variables|Default|SetIntermissionCheck true)
      (Variables|Default|SetWaveActive false)
      (Audio|PlaySound2D "/Game/FPSK/Sounds/WAV_SuccessJingleElectric.WAV_SuccessJingleElectric" 3.0)
      (Variables|Default|SetCompleteString " COMPLETE")
      (CallFunction|WaveDisplayPlayAnimation))))

(event Custom|BeginIntermission
  ;[0 0 0] Intermission Timer
  (Variables|Default|SetIntermissionSeconds 60)
  (Variables|Default|SetIntermission true)
  ;;[1 1 1] Intermission countdown timer loop
  (Utilities|FlowControl|Delay 1.0 :!label _label)
  (if (Variables|Default|GetIntermission)
    (bind _result (Math|Integer|DecrementInt (Variables|Default|GetIntermissionSeconds))
      (:%20%20
        (Math|Integer|CompareInt _result
          (:>
            (goto _label))
          (:==
            _)
          (:<
            _))
        (CallFunction|BeginNextWave)))))

(event EventBeginPlay
  ;[0 0 0] Begin Play
  ;;[1 1 1] Delay for good measure required to allow HUD to spawn
  (Utilities|FlowControl|Delay 0.0)
  ;;[1 1 1] Get Player Character
  (CallFunction|SetPlayerCharacters)
  ;;[1 1 1] Get and set Zombie Spawn points
  (bind _outactors (Actor|GetAllActorsOfClass "/Game/FPSK/Blueprint/ZombieGameMode/BP_ZombieSpawnPoint.BP_ZombieSpawnPoint_C"))
  (Variables|Default|SetZombieSpawnPoints _outactors)
  ;;[1 1 1] Begin first wave
  (CallFunction|BeginNextWave))

(fn ConstructionScript)

(fn SetPlayerCharacters
  (bind _outactors (Actor|GetAllActorsOfClass "/Game/FPSK/FirstPersonAssets/FirstPersonBP/Blueprints/FirstPersonCharacter.FirstPersonCharacter_C"))
  (Variables|Default|SetPlayerCharacter _outactors))

(fn SetSpawnLocationArray
  (Utilities|Array|Clear (Variables|Default|GetAvailableSpawnLocations))
  (for _array_element (Variables|Default|GetZombieSpawnPoints)
    (if (Variables|/Game/FPSK/Blueprint/ZombieGameMode/BP_ZombieSpawnPoint.BP_ZombieSpawnPoint_C|GetCanSpawn _array_element)
      (Utilities|Array|Add (Variables|Default|GetAvailableSpawnLocations) (Variables|/Game/FPSK/Blueprint/ZombieGameMode/BP_ZombieSpawnPoint.BP_ZombieSpawnPoint_C|GetSpawnLocation _array_element)))))

(fn WaveDisplayPlayAnimation
  (CallFunction|SetPlayerCharacters)
  (for _array_element (Variables|Default|GetPlayerCharacter)
    (Utilities|IsValid (Variables|/Game/FPSK/FirstPersonAssets/FirstPersonBP/Blueprints/FirstPersonCharacter.FirstPersonCharacter_C|GetMainHUD _array_element)
      (:Is%20Valid
        (Default|WavePlayAnimation (Variables|/Game/FPSK/FirstPersonAssets/FirstPersonBP/Blueprints/FirstPersonCharacter.FirstPersonCharacter_C|GetMainHUD _array_element))))))