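; Zombie-mode mystery crate that opens to reveal a random gun pickup from its weapon pool.
; OpenMysteryCrate spawns a floating pickup, then ChangeGun re-rolls it on a timeline-driven delay until it becomes collectable and repurchase unlocks.
; An unclaimed gun is destroyed after a timeout; Tick interpolates lid, light and audio, closing the crate once the pickup is gone.
; An editor-called event fills the pool from gun pickups placed in the level.
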(event Custom|Add%20All%20Level%20Weapons
  ;[0 0 0] Adds all guns from level into Weapon Pool (Call from editor)
  (bind _outactors (Actor|GetAllActorsOfClass "/Game/FPSK/Blueprint/BP_GunPickup.BP_GunPickup_C"))
  (for _array_element _outactors
    (Utilities|Array|AddUnique (Variables|WeaponPool|GetWeaponListPool) (Variables|/Game/FPSK/Blueprint/BP_GunPickup.BP_GunPickup_C|GetWeaponVariables _array_element))))

(event Custom|OpenMysteryCrate
  (bind _weaponlistpool (Variables|WeaponPool|GetWeaponListPool))
  ;[0 0 0] Open Mystery Crate
  ;;[1 1 1] If there is a gun already destroy the gun
  (Utilities|IsValid (Variables|Default|GetGunPickup)
    (:Is%20Valid
      (Actor|DestroyActor (Variables|Default|GetGunPickup)))
    (:Is%20Not%20Valid
      _))
  ;;[1 1 1] Make unpurchasable until gun is revealed
  (Variables|Default|SetCanPurchase false)
  ;;[1 1 1] Open chest
  (Variables|Default|SetChestOpenTarget 1.0)
  ;;[1 1 1] Gun wont be destroyed from Destroy Gun Timer
  (Variables|Default|SetDestroyGunTimer false)
  ;;[1 1 1] Start timelines
  (CallFunction|PlayGunPickupAnimations)
  (CallFunction|PlayGunChangeSpeedTimeline)
  ;;[1 1 1] Spawn a gun
  (bind _returnvalue (Game|SpawnActorfromClass "/Game/FPSK/Blueprint/BP_GunPickup.BP_GunPickup_C" (Transformation|GetWorldTransform (Variables|Default|GetGunFloatLocation)) "Undefined" 0 (Utilities|Array|Get(acopy) _weaponlistpool (Math|Random|RandomIntegerinRange 0 (- (Utilities|Array|Length _weaponlistpool) 1))) false true false false false 0))
  ;;[1 1 1] Set and attach to scene component
  (bind _output_get (Variables|Default|SetGunPickup _returnvalue))
  (Transformation|AttachComponentToComponent _output_get (Variables|Default|GetGunFloatLocation) "None" "SnapToTarget" "SnapToTarget" "SnapToTarget" true)
  ;;[1 1 1] Start gun change loop
  (Variables|Default|SetChangeGunLoop true)
  (CallFunction|ChangeGun))

(event Custom|PlayGunPickupAnimations
  (bind _gunfloatlocation (Variables|Default|GetGunFloatLocation))
  (bind _relativelocation (Variables|/Script/Engine.SceneComponent|GetRelativeLocation _gunfloatlocation))
  (bind (_x _y) (Math|Vector|BreakVector _relativelocation))
  ;[0 0 0] Gun Float animation
  (Utilities|FlowControl|Sequence
    (:then_0
      (bind _zfloat (Timeline|FloatTimeline PlayFromStart)
        (:Update
          (Transformation|SetRelativeLocation _gunfloatlocation (Math|Vector|MakeVector _x _y (+ (* _zfloat 1e+01) (Math|Float|Lerp 5.0 (Variables|Default|GetInitialZLocation) (stale _popuplerp)))) false false))))
    (:then_1
      (bind _popuplerp (Timeline|PopupTimeline PlayFromStart)))))

(event Custom|StopFloatAnimation
  (bind _gunfloatlocation (Variables|Default|GetGunFloatLocation))
  (bind _relativelocation (Variables|/Script/Engine.SceneComponent|GetRelativeLocation _gunfloatlocation))
  (bind (_x _y) (Math|Vector|BreakVector _relativelocation))
  ;[0 0 0] Gun Float animation
  (bind _zfloat (Timeline|FloatTimeline Stop)
    (:Update
      (Transformation|SetRelativeLocation _gunfloatlocation (Math|Vector|MakeVector _x _y (+ (* _zfloat 1e+01) (Math|Float|Lerp 5.0 (Variables|Default|GetInitialZLocation) (stale Custom|PlayGunPickupAnimations _popuplerp)))) false false))))

(event Custom|ChangeGun
  (bind _weaponlistpool (Variables|WeaponPool|GetWeaponListPool))
  (bind _gunpickup (Variables|Default|GetGunPickup))
  ;[0 0 0] Change gun
  ;;[1 1 1] Play sound every time the gun changes
  (Audio|PlaySoundatLocation "/Game/FPSK/Sounds/CUE_BulletCaseImpact.CUE_BulletCaseImpact" (Transformation|GetWorldLocation (Variables|Default|GetGunFloatLocation)))
  ;;[1 1 1] Construct gun from random weapon in WeaponPool
  (Variables|/Game/FPSK/Blueprint/BP_GunPickup.BP_GunPickup_C|SetWeaponVariables _gunpickup (Utilities|Array|Get(acopy) _weaponlistpool (Math|Random|RandomIntegerinRange 0 (- (Utilities|Array|Length _weaponlistpool) 1))))
  (Default|GunConstruct _gunpickup)
  ;;[1 1 1] Loop gun change
  (if (Variables|Default|GetChangeGunLoop)
    (Utilities|FlowControl|Delay (Variables|Default|GetGunChangeLoopDelay))
    (CallFunction|ChangeGun)
    (else
      ;[0 0 0] After the resulting gun is revealed
      ;;[1 1 1] Allow gun to be picked up
      (Variables|/Game/FPSK/Blueprint/BP_GunPickup.BP_GunPickup_C|SetPickupActive (Variables|Default|GetGunPickup) true)
      ;;[1 1 1] Able to repurchase Mystery Crate
      (Variables|Default|SetCanPurchase true)
      ;;[1 1 1] Destroy gun timer
      (Variables|Default|SetDestroyGunTimer true)
      (Utilities|FlowControl|RetriggerableDelay 1e+01) ; Seconds to decide if you want to pick up resulting gun
      (if (Variables|Default|GetDestroyGunTimer)
        (Utilities|IsValid (Variables|Default|GetGunPickup)
          (:Is%20Valid
            (Actor|DestroyActor (Variables|Default|GetGunPickup))
            ;;[1 1 1] Close crate
            (Variables|Default|SetChestOpenTarget 0.0)))))))

(event Custom|PlayGunChangeSpeedTimeline
  ;[0 0 0] Decrease Gun Change Loop Delay over time, Stop loop when finished
  (bind _newtrack_1 (Timeline|GunChangeSpeed PlayFromStart)
    (:Update
      (Variables|Default|SetGunChangeLoopDelay (Math|Float|Lerp 1.0 0.1 _newtrack_1)))
    (:Finished
      (Variables|Default|SetChangeGunLoop false))))

(event EventTick
  (params (DeltaSeconds :type Float%20%28single-precision%29))
  (Utilities|FlowControl|Sequence
    (:then_0
      ;[0 0 0] Open/Close lid
      ;;[1 1 1] If chest open value is not at target
      (if (!= (Variables|Default|GetChestOpenValue) (Variables|Default|GetChestOpenTarget))
        ;;[1 1 1] Interpolate to chest open target
        (bind _output_get (Variables|Default|SetChestOpenValue (Math|Interpolation|FInterpTo (Variables|Default|GetChestOpenValue) (Variables|Default|GetChestOpenTarget) (Utilities|Time|GetWorldDeltaSeconds) 5.0)))
        ;;[1 1 1] Set Lid rotation based on chest open value
        (Transformation|SetRelativeRotation (Variables|Default|GetMysteryCrateLid) (Math|Rotator|Lerp(Rotator) "0, 0, 0" "0, 0,-130.000000" _output_get true) false false)
        ;;[1 1 1] Set light intensity
        (Rendering|Components|Light|SetIntensity (Variables|Default|GetPointLight) (* (Variables|Default|GetChestOpenValue) (Variables|Default|GetLightIntensity)))
        ;;[1 1 1] Adjust MysteryCrate audio volume
        (Audio|Components|Audio|SetVolumeMultiplier (Variables|Default|GetMysteryCrateLoop) (Variables|Default|GetChestOpenValue) :!class /Script/Engine.AudioComponent)
        (Utilities|FlowControl|Sequence
          (:then_0
            ;[0 0 0] Sounds
            ;;[1 1 1] Sound on Shut
            (if (and (Math|Float|NearlyEqual(Float) (Variables|Default|GetChestOpenValue) 0.0 0.01) (== (Variables|Default|GetChestOpenTarget) 0.0))
              (Utilities|FlowControl|DoOnce false :!label _label
                (:Completed
                  (Audio|PlaySoundatLocation "/Game/FPSK/Sounds/WAV_ChestShut.WAV_ChestShut" (Transformation|GetActorLocation) "0, 0, 0" 1.0 0.8 0.0 "/Game/FPSK/Sounds/Audio/Attenuation_MediumRange.Attenuation_MediumRange")))
              (else
                (goto _label Reset))))
          (:then_1
            ;;[1 1 1] Sound on Open
            (if (and (Math|Float|NearlyEqual(Float) (Variables|Default|GetChestOpenValue) 0.0 0.1) (== (Variables|Default|GetChestOpenTarget) 1.0))
              (Utilities|FlowControl|DoOnce false :!label _label_2
                (:Completed
                  (Audio|PlaySoundatLocation "/Game/FPSK/Sounds/WAV_ChestOpen.WAV_ChestOpen" (Transformation|GetActorLocation) "0, 0, 0" 2.0 1.0 0.0 "/Game/FPSK/Sounds/Audio/Attenuation_MediumRange.Attenuation_MediumRange")))
              (else
                (goto _label_2 Reset))))
          (:then_2
            ;;[1 1 1] Sound on Close
            (if (and (Math|Float|NearlyEqual(Float) (Variables|Default|GetChestOpenValue) 1.0 0.1) (== (Variables|Default|GetChestOpenTarget) 0.0))
              (Utilities|FlowControl|DoOnce false :!label _label_3
                (:Completed
                  (Audio|PlaySoundatLocation "/Game/FPSK/Sounds/WAV_ChestSqueak.WAV_ChestSqueak" (Transformation|GetActorLocation) "0, 0, 0" 1.0 1.0 0.0 "/Game/FPSK/Sounds/Audio/Attenuation_MediumRange.Attenuation_MediumRange")))
              (else
                (goto _label_3 Reset)))))))
    (:then_1
      ;[0 0 0] If GunPickup is picked up or destroyed, close chest
      (Utilities|IsValid (Variables|Default|GetGunPickup)
        (:Is%20Not%20Valid
          (Variables|Default|SetChestOpenTarget 0.0))))))

(fn ConstructionScript
  ;[0 0 0] Set initial Z location of Gun Float Location
  (Variables|Default|SetInitialZLocation (.Z (Math|Vector|BreakVector (Variables|/Script/Engine.SceneComponent|GetRelativeLocation (Variables|Default|GetGunFloatLocation))))))