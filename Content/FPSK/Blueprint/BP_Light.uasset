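; Configurable light fixture that can break when damaged, dangling from a cable and flickering.
; The construction script applies radius, intensity and color to the point light and emissive material, then runs an editor alignment tool.
; Damage on destructible lights triggers a one-time break into constrained physics with crackle sound and an endless, randomly timed flicker loop.
; Lights flagged Destroyed break on BeginPlay with a random impulse.
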(event Custom|LightFlicker
  ;[0 0 0] Light Flicker logic
  ;;[1 1 1] If light is on
  (if (> (Variables|/Script/Engine.LightComponentBase|GetIntensity (Variables|Default|GetPointLight)) 0.0)
    ;;[1 1 1] Shut off
    (Rendering|Material|SetScalarParameterValueonMaterials (Variables|Default|GetLight) "LightPower" 0.0)
    (Rendering|Components|Light|SetIntensity (Variables|Default|GetPointLight) 0.0)
    (else
      ;;[1 1 1] Turn on
      (Rendering|Material|SetScalarParameterValueonMaterials (Variables|Default|GetLight) "LightPower" (* (Variables|LightSettings|GetLightIntensity) 0.01))
      (Rendering|Components|Light|SetIntensity (Variables|Default|GetPointLight) (Variables|LightSettings|GetLightIntensity))
      (Audio|PlaySoundatLocation "/Game/FPSK/Sounds/WAV_LightSwitch.WAV_LightSwitch" (Transformation|GetActorLocation) "0, 0, 0" 1.0 1.0 0.0 "/Game/FPSK/Sounds/Audio/Attenuation_MediumRange.Attenuation_MediumRange")))
  (Utilities|FlowControl|Delay (Math|Random|RandomFloatinRange 0.05 0.2))
  (CallFunction|LightFlicker))

(event Custom|DestroyLight
  ;[0 0 0] Destruction events
  ;;[1 1 1] Break light = spawn cable, flicker on/off and simulate physics
  (Utilities|FlowControl|DoOnce false
    (:Completed
      (CallFunction|BreakLight)
      (CallFunction|LightFlicker))))

(event EventBeginPlay
  ;[0 0 0] Begin Play events
  ;;[1 1 1] If destroyed, break light
  (if (Variables|LightSettings|GetDestroyed)
    (CallFunction|DestroyLight)
    ;;[1 1 1] Close break gate
    (Variables|Default|SetCloseBreakGate true)
    ;;[1 1 1] Randomly shake light physics
    (Physics|AddRadialImpulse (Variables|Default|GetLight) (+ (Transformation|GetWorldLocation (Variables|Default|GetLight)) (Math|Vector|MakeVector (Math|Random|RandomFloatinRange -1e+01 1e+01) (Math|Random|RandomFloatinRange -1e+01 1e+01) (Math|Random|RandomFloatinRange -1e+01 1e+01))) 5e+01 5e+01 "RIF_Constant" true)))

(event Game|Damage|EventPointDamage
  (params (Damage :type Float%20%28single-precision%29) (DamageType :type Damage%20Type%20Object%20Reference) (HitLocation :type Vector :default "0, 0, 0") (HitNormal :type Vector :default "0, 0, 0") (HitComponent :type Primitive%20Component%20Object%20Reference) (BoneName :type Name :default "None") (ShotFromDirection :type Vector :default "0, 0, 0") (InstigatedBy :type Controller%20Object%20Reference) (DamageCauser :type Actor%20Object%20Reference) (HitInfo :type Hit%20Result%20Structure%20%28by%20ref%29))
  ;[0 0 0] Destruction events
  (if (Variables|LightSettings|GetDestructable)
    (CallFunction|DestroyLight)))

(event Game|Damage|EventAnyDamage
  (params (Damage :type Float%20%28single-precision%29) (DamageType :type Damage%20Type%20Object%20Reference) (InstigatedBy :type Controller%20Object%20Reference) (DamageCauser :type Actor%20Object%20Reference))
  ;[0 0 0] Destruction events
  (if (Variables|LightSettings|GetDestructable)
    (CallFunction|DestroyLight)))

(fn ConstructionScript
  (bind _lightcolor (Variables|LightSettings|GetLightColor))
  (bind (_r _g _b) (Utilities|Struct|BreakLinearColor _lightcolor))
  (Utilities|FlowControl|Sequence
    (:then_0
      ;[0 0 0] Construct Light
      ;;[1 1 1] Set light settings
      (Rendering|Lighting|SetAttenuationRadius (Variables|Default|GetPointLight) (Variables|LightSettings|GetLightRadius))
      (Rendering|Components|Light|SetIntensity (Variables|Default|GetPointLight) (Variables|LightSettings|GetLightIntensity))
      (Rendering|Components|Light|SetLightColor (Variables|Default|GetPointLight) (Variables|LightSettings|GetLightColor) true)
      ;;[1 1 1] Set color and emissive power in material
      (Rendering|Material|SetScalarParameterValueonMaterials (Variables|Default|GetLight) "LightPower" (* (Variables|LightSettings|GetLightIntensity) 0.01))
      (Rendering|Material|SetVectorParameterValueonMaterials (Variables|Default|GetLight) "LightColor" (Math|Vector|MakeVector _r _g _b)))
    (:then_1
      ;[0 0 0] Alignment tool for easy alignment in editor
      (Utilities|AlignTool (Variables|AlignmentTool|GetAlignToReference) (Variables|AlignmentTool|GetAlignment)))))

(fn BreakLight
  (bind _physicsconstraint (Variables|Default|GetPhysicsConstraint))
  (bind _cordlength (Variables|LightSettings|GetCordLength))
  ;[0 0 0] Break light function
  ;;[1 1 1] Simulate physics of light
  (Physics|SetSimulatePhysics (Variables|Default|GetLight) true)
  ;;[1 1 1] Set physics constraint length
  (Class|PhysicsConstraintComponent|SetLinearXLimit _physicsconstraint "LCM_Limited" _cordlength)
  (Class|PhysicsConstraintComponent|SetLinearYLimit _physicsconstraint "LCM_Limited" _cordlength)
  (Class|PhysicsConstraintComponent|SetLinearZLimit _physicsconstraint "LCM_Limited" _cordlength)
  ;;[1 1 1] Add cable
  (AddComponent|AddCableComponent false)
  ;;[1 1 1] Play sound
  (Audio|PlaySoundatLocation "/Game/FPSK/Sounds/WAV_Electric_Crackle.WAV_Electric_Crackle" (Transformation|GetActorLocation) "0, 0, 0" 1.0 1.0 0.0 "/Game/FPSK/Sounds/Audio/Attenuation_MediumRange.Attenuation_MediumRange"))